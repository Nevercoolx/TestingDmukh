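; BP_Drawing is an interactable, inspectable drawing with two clickable inspect points.
; Interact reveals both points and StopInspection hides them.
; Clicking the first point only plays a sound.
; Clicking the second plays another sound, tells the player's interaction component to stop inspecting, hides the points and sends a notification to the main widget.
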(event `self.ReceiveBeginPlay`
  (set `self.Inspect Points` (`|MakeArray` (`self.Inspect1`) (`self.Inspect2`))))

(event `/Game/Core/Interaction/BPI_Interactble.Interact`
  (params (Interactor :type "Actor Object Reference"))
  (for _array_element (`self.Inspect Points`)
    (`SceneComponent.SetVisibility` _array_element true false)))

(event `self.Inspect1.OnClicked`
  (params (TouchedComponent :type "PrimitiveComponent Object Reference") (ButtonPressed :type "Key Structure"))
  (`GameplayStatics.PlaySound2D` "/Game/Core/Sounds/Ordena.Ordena" 1.0 1.0 0.0 null null))

(event `self.Inspect2.OnClicked`
  (params (TouchedComponent :type "PrimitiveComponent Object Reference") (ButtonPressed :type "Key Structure"))
  (`GameplayStatics.PlaySound2D` "/Game/Core/Sounds/Вжух.Вжух" 1.0 1.0 0.0 null null)
  (message `/Game/Core/Interaction/BPI_Interactble.StopInspecting` (`self.GetComponentByClass` (`GameplayStatics.GetPlayerCharacter` 0) "/Game/Core/Interaction/PlayerInteractionComp.PlayerInteractionComp_C"))
  (for _array_element (`self.Inspect Points`)
    (`SceneComponent.SetVisibility` _array_element false false))
  (bind _foundwidgets (`WidgetBlueprintLibrary.GetAllWidgetsOfClass` "/Game/Core/UI/Widgets/W_MainWidget.W_MainWidget_C"))
  (message `/Game/Core/UI/Blueprints/BPI_MasterHUD.UpdateNotifications` _foundwidgets (`self.Notification`)))

(event `/Game/Core/Interaction/BPI_Interactble.StopInspection`
  (for _array_element (`self.Inspect Points`)
    (`SceneComponent.SetVisibility` _array_element false false)))

(fn `UserConstructionScript`)