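; BP_Vase is an inspectable vase that the player can examine and rotate, with clickable inspection points.
; Interact hides the world mesh, shows Sphere1, sets the character's ChildActor to a vase copy and enables rotation on PlayerInteractionComp.
; Clicking Sphere1 posts a remark to W_MainWidget.
; StopInspection clears the copy, restores the mesh, disables rotation, hides the points and updates the notification.
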(event `self.ReceiveBeginPlay`
  (set `self.InspectPoints` (`|MakeArray` (`self.Sphere1`) null)))

(event `/Game/Core/Interaction/BPI_Interactble.Interact`
  (params (Interactor :type "Actor Object Reference"))
  (bind _foundwidgets (`WidgetBlueprintLibrary.GetAllWidgetsOfClass` "/Game/Core/UI/Widgets/W_MainWidget.W_MainWidget_C"))
  (set `self.MainWidget` _foundwidgets)
  (`SceneComponent.SetVisibility` (`self.Sphere1`) true false)
  (bind _asbp_third_person_character (cast `/Game/ThirdPerson/Blueprints/BP_ThirdPersonCharacter` Interactor))
  (bind _output_get (set `self.As BP Third Person Character` _asbp_third_person_character))
  (bind _childactor (`/Game/ThirdPerson/Blueprints/BP_ThirdPersonCharacter.ChildActor` _output_get))
  (`ChildActorComponent.SetChildActorClass` _childactor "BP_Vase_C")
  (`SceneComponent.SetVisibility` _childactor true false)
  (`SceneComponent.SetVisibility` (`self.StaticMesh`) false false)
  (set `/Game/Core/Interaction/PlayerInteractionComp.CanBeRotated` true (`self.GetComponentByClass` (`self.As BP Third Person Character`) "/Game/Core/Interaction/PlayerInteractionComp.PlayerInteractionComp_C")))

(event `/Game/Core/Interaction/BPI_Interactble.StopInspection`
  (`ChildActorComponent.SetChildActorClass` (`/Game/ThirdPerson/Blueprints/BP_ThirdPersonCharacter.ChildActor` (`self.As BP Third Person Character`)) null)
  (`SceneComponent.SetVisibility` (`self.StaticMesh`) true false)
  (set `/Game/Core/Interaction/PlayerInteractionComp.CanBeRotated` false (`self.GetComponentByClass` (`self.As BP Third Person Character`) "/Game/Core/Interaction/PlayerInteractionComp.PlayerInteractionComp_C"))
  (for _array_element (`self.InspectPoints`)
    (`SceneComponent.SetVisibility` _array_element false false))
  (message `/Game/Core/UI/Blueprints/BPI_MasterHUD.UpdateNotifications` (`self.MainWidget`) (`self.Notification`)))

(event `self.Sphere1.OnClicked`
  (params (TouchedComponent :type "PrimitiveComponent Object Reference") (ButtonPressed :type "Key Structure"))
  (message `/Game/Core/UI/Blueprints/BPI_MasterHUD.UpdateNotifications` (`self.MainWidget`) "Вроде ваза как ваза."))

(fn `ShowPoints`
  (for _array_element (`self.InspectPoints`)
    (`SceneComponent.SetVisibility` _array_element true false)))

(fn `UserConstructionScript`
  (`StaticMeshComponent.SetStaticMesh` (`self.StaticMesh`) (`self.ItemModel`)))