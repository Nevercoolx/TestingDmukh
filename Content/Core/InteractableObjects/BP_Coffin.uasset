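; BP_Coffin is an inspectable coffin with clickable hotspots that play sounds and lead to loot notifications.
; Interact reveals Inspect1 and Inspect3 and sweeps the interactor toward world origin; InspectionFinished hides both and notifies PlayerInteractionComp.
; Inspect1 reveals Inspect2, which shifts StaticMesh1, destroys itself, ends inspection and reports loot through W_MainWidget.
; Once Inspect2 is gone, Inspect1 reports no loot; Inspect3 only plays a sound.
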(event `self.ReceiveBeginPlay`
  (set `self.InspectPoints` (`|MakeArray` (`self.Inspect1`) (`self.Inspect3`))))

(event `/Game/Core/Interaction/BPI_Interactble.Interact`
  (params (Interactor :type "Actor Object Reference"))
  (for _array_element (`self.InspectPoints`)
    (`SceneComponent.SetVisibility` _array_element true false)
    (`self.K2_SetActorLocation` Interactor (0.0 0.0 0.0) true false)))

(event `self.Inspect1.OnClicked`
  (params (TouchedComponent :type "PrimitiveComponent Object Reference") (ButtonPressed :type "Key Structure"))
  (`/Engine/EditorBlueprintResources/StandardMacros.IsValid` (`self.Inspect2`)
    (:`Is Valid`
      (`GameplayStatics.PlaySound2D` "/Game/Core/Sounds/гроб.гроб" 1.0 1.0 0.0 null null)
      (`SceneComponent.SetVisibility` (`self.Inspect2`) true false))
    (:`Is Not Valid`
      (bind _foundwidgets (`WidgetBlueprintLibrary.GetAllWidgetsOfClass` "/Game/Core/UI/Widgets/W_MainWidget.W_MainWidget_C"))
      (message `/Game/Core/UI/Blueprints/BPI_MasterHUD.UpdateNotifications` _foundwidgets (`self.NotificationNoLoot`)))))

(event `self.Inspect3.OnClicked`
  (params (TouchedComponent :type "PrimitiveComponent Object Reference") (ButtonPressed :type "Key Structure"))
  (`GameplayStatics.PlaySound2D` "/Game/Core/Sounds/Резьба.Резьба" 1.0 1.0 0.0 null null))

(event `self.Inspect2.OnClicked`
  (params (TouchedComponent :type "PrimitiveComponent Object Reference") (ButtonPressed :type "Key Structure"))
  (`SceneComponent.K2_SetRelativeLocation` (`self.StaticMesh1`) (-50.0 0.0 100.0) false false)
  (`GameplayStatics.PlaySound2D` "/Game/Core/Sounds/Сдвинули.Сдвинули" 1.0 1.0 0.0 null null)
  (`ActorComponent.K2_DestroyComponent` (`self.Inspect2`))
  (`self.InspectionFinished`)
  (bind _foundwidgets (`WidgetBlueprintLibrary.GetAllWidgetsOfClass` "/Game/Core/UI/Widgets/W_MainWidget.W_MainWidget_C"))
  (message `/Game/Core/UI/Blueprints/BPI_MasterHUD.UpdateNotifications` _foundwidgets (`self.NotificationLoot`)))

(event `/Game/Core/Interaction/BPI_Interactble.StopInspection`
  (`self.InspectionFinished`))

(fn `InspectionFinished`
  (message `/Game/Core/Interaction/BPI_Interactble.StopInspecting` (`self.GetComponentByClass` (`GameplayStatics.GetPlayerCharacter` 0) "/Game/Core/Interaction/PlayerInteractionComp.PlayerInteractionComp_C"))
  (for _array_element (`self.InspectPoints`)
    (`SceneComponent.SetVisibility` _array_element false false)))

(fn `UserConstructionScript`)